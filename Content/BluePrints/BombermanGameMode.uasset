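; Game mode for a Bomberman-style game that shows the main UI and handles the end-of-match screen.
; On BeginPlay it creates the MainUserInterface widget, adds it to the viewport and calls StartGame.
; Its TriggerGameOver override calls the parent, then writes the winning player number or a draw to the UI.
; A short timer then calls FreezeGame, which pauses the game, shows the cursor and restart button, and switches to UI-only input.
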(event Custom|FreezeGame
  (bind _returnvalue (Game|GetPlayerController 0))
  (Input|SetInputModeUIOnly _returnvalue (Variables|Default|GetMainUI) "DoNotLock")
  (Variables|/Script/Engine.PlayerController|SetbShowMouseCursor _returnvalue true)
  (Widget|SetVisibility (Variables|/Game/UserInterface/MainUserInterface.MainUserInterface_C|GetRestartButton (Variables|Default|GetMainUI)) "Visible")
  (Game|SetGamePaused true))

(event EventBeginPlay
  (bind _returnvalue (UserInterface|CreateWidget "/Game/UserInterface/MainUserInterface.MainUserInterface_C"))
  (bind _output_get (Variables|Default|SetMainUI _returnvalue))
  (UserInterface|Viewport|AddtoViewport _output_get 0)
  (Class|BombermanTestGameModeBase|StartGame))

(event EventTick
  (params (DeltaSeconds :type Float%20%28single-precision%29)))

(fn ConstructionScript)

(fn TriggerGameOver
  (params (numAlivePlayers :type Integer) (winner :type Bomberman%20Player%20Object%20Reference))
  (bind _mainui (Variables|Default|GetMainUI))
  (bind _resulttext (Variables|/Game/UserInterface/MainUserInterface.MainUserInterface_C|GetResultText _mainui))
  (|CallParentFunction numAlivePlayers winner)
  (if (and (> numAlivePlayers 0) (Utilities|IsValid winner))
    (Rendering|Components|TextRender|SetText _resulttext (Utilities|Text|ToText(String) (Utilities|String|BuildString(Integer) "" "Player " (+ (Variables|/Script/BombermanTest.BombermanPlayer|GetplayerNum winner) 1) " wins!")))
    (else
      (Rendering|Components|TextRender|SetText _resulttext "DRAW")))
  (Utilities|Time|SetTimerbyFunctionName 0 "FreezeGame" 0.1))